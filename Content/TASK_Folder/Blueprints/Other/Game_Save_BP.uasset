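; Game_Save_BP is a data holder for the player's game settings, covering display, graphics quality, audio and key mappings.
; Individual Save events each store one value in its own variable.
; Save_Game_Settings either takes a whole settings struct or rebuilds it from those variables, depending on a flag, so single changes reach GameSettings only when it runs.
; Getters return the combined struct and the key mappings; no disk writing happens here.
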(event `Save_Game_Settings`
  (params (`new value` :type "/Game/TASK_Folder/Blueprints/Struct/Game_Setings Structure") (With_New_Param :type Boolean))
  ;[1 1 1] Save Functions
  (if With_New_Param
    (set `self.Game_Settings` `new value`)
    (else
      (set `self.Game_Settings` (make `/Game/TASK_Folder/Blueprints/Struct/Game_Setings` (`self.Window_Mode`) (`self.Display_Resolution`) (`self.Frame_Rate_Limit`) (`self.View Distance`) (`self.Post Processing`) (`self.Anti Aliasing`) (`self.Texture Quality`) (`self.Shadow Quality`) (`self.Grass`) (`self.Master Volume`) (`self.Music Volume`) (`self.SFX Volume`) (`self.Dialogue Volume`) (`self.Audio Output Mode`) (`self.Key_Mappings`))))))

(event `Save_Grass`
  (params (`new value` :type "/Game/TASK_Folder/Blueprints/Enums/Settings_Grade Enum" :default "NewEnumerator0"))
  ;[1 1 1] Save Functions
  (set `self.Grass` `new value`))

(event `Save_SFX_Volume`
  (params (`new value` :type "Float (double-precision)"))
  ;[1 1 1] Save Functions
  (set `self.SFX Volume` `new value`))

(event `Save_Post_Processing`
  (params (`new value` :type "/Game/TASK_Folder/Blueprints/Enums/Settings_Grade Enum" :default "NewEnumerator0"))
  ;[1 1 1] Save Functions
  (set `self.Post Processing` `new value`))

(event `Save_Dialogue_Volume`
  (params (`new value` :type "Float (double-precision)"))
  ;[1 1 1] Save Functions
  (set `self.Dialogue Volume` `new value`))

(event `Save_Anti_Aliasing`
  (params (`new value` :type "/Game/TASK_Folder/Blueprints/Enums/Settings_Grade Enum" :default "NewEnumerator0"))
  ;[1 1 1] Save Functions
  (set `self.Anti Aliasing` `new value`))

(event `Save_Audio_Output_Mode`
  (params (`new value` :type String))
  ;[1 1 1] Save Functions
  (set `self.Audio Output Mode` `new value`))

(event `Save_Texture_Quality`
  (params (`new value` :type "/Game/TASK_Folder/Blueprints/Enums/Settings_Grade Enum" :default "NewEnumerator0"))
  ;[1 1 1] Save Functions
  (set `self.Texture Quality` `new value`))

(event `Save_Window_Mode`
  (params (NewParam :type "/Game/TASK_Folder/Blueprints/Enums/Screen_Mode Enum" :default "NewEnumerator0"))
  ;[1 1 1] Save Functions
  (set `self.Window_Mode` NewParam))

(event `Save_Shadow_Quality`
  (params (`new value` :type "/Game/TASK_Folder/Blueprints/Enums/Settings_Grade Enum" :default "NewEnumerator0"))
  ;[1 1 1] Save Functions
  (set `self.Shadow Quality` `new value`))

(event `Save_Key_Mappings`
  (params (New_Value :type "Array of EnhancedActionKeyMapping Structure"))
  ;[1 1 1] Save Functions
  (set `self.Key_Mappings` New_Value))

(event `Save_Display_Resolution`
  (params (`new value` :type "/Game/TASK_Folder/Blueprints/Enums/Resolution_Grade Enum" :default "NewEnumerator0"))
  ;[1 1 1] Save Functions
  (set `self.Display_Resolution` `new value`))

(event `Save_View_Distance`
  (params (`new value` :type "/Game/TASK_Folder/Blueprints/Enums/Settings_Grade Enum" :default "NewEnumerator0"))
  ;[1 1 1] Save Functions
  (set `self.View Distance` `new value`))

(event `Save_Frame_Rate_Limit`
  (params (`new value` :type "/Game/TASK_Folder/Blueprints/Enums/Frame_Rate_Limit Enum" :default "NewEnumerator0"))
  ;[1 1 1] Save Functions
  (set `self.Frame_Rate_Limit` `new value`))

(event `Save_Master_Volume`
  (params (`new value` :type "Float (double-precision)"))
  ;[1 1 1] Save Functions
  (set `self.Master Volume` `new value`))

(event `Save_Music_Volume`
  (params (`new value` :type "Float (double-precision)"))
  ;[1 1 1] Save Functions
  (set `self.Music Volume` `new value`))

(fn `Get_Game_Settings`
  (returns (Result :type "/Game/TASK_Folder/Blueprints/Struct/Game_Setings Structure"))
  (return (`self.Game_Settings`)))

(fn `Get_Inputs`
  (returns (`Inputs Result` :type "Array of EnhancedActionKeyMapping Structure"))
  (return (`self.Key_Mappings`)))