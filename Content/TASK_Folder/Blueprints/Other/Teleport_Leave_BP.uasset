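; Quest-gated marker actor, named as a teleport exit, that shows a Niagara effect when its requested quest is the player's current one.
; On BeginPlay it caches the QuestSystem from the player's custom controller and compares quest IDs.
; A match adds and stores the Niagara component, otherwise any stored one is destroyed.
; The check runs only once, and the graph contains no overlap or teleport logic.
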(event `self.ReceiveBeginPlay`
  ;[1 1 1] On begin spawn it if  Current quest is same with request quest, and also on begin get and save the player quest system component.
  (bind _ascustom_controller_bp (cast `/Game/TASK_Folder/Blueprints/Character/Custom_Controller_BP` (`GameplayStatics.GetPlayerController` 0)))
  (bind _quest_system (`Custom_Player_Controller_PR.Quest_System` _ascustom_controller_bp))
  (set `self.Quest System` _quest_system)
  (if (`KismetStringLibrary.EqualEqual_StrStr` (`.Quest_ID` (break `Quest_Data` (`self.Requested_Quest_Data`))) (`.Quest_ID` (break `Quest_Data` (`Quest_System_Component_PR.Get_Current_Quest_Data` _quest_system))))
    (bind _returnvalue (`AddComponent|NODE_AddNiagaraComponent-0` :`RelativeTransform` (`SceneComponent.GetRelativeTransform` (`self.DefaultSceneRoot`))))
    (set `self.Created_Niagara_System` _returnvalue)
    (else
      (bind _created_niagara_system (`self.Created_Niagara_System`)
        (:`then`
          (`ActorComponent.K2_DestroyComponent` _created_niagara_system))
        (:`else`)))))

(fn `UserConstructionScript`)