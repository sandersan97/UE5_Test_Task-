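; Magic projectile actor that, on hit, swaps its Niagara effect to an explosion, deals damage to the hit actor and destroys itself after a short delay.
; The hit also checks the player controller's quest system and triggers interaction on Quest_Obj actors implementing the interact interface.
; That interaction is hardcoded to two unfinished locations of the "Last Trouble" quest, matched against the current quest data.
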(event `Start_Hit`
  (params (Hit_Result :type "HitResult Structure"))
  (bind (_bblockinghit _binitialoverlap _time _distance _location _impactpoint _normal _impactnormal _physmat _hitactor _hitcomponent) (`GameplayStatics.BreakHitResult` Hit_Result))
  ;[1 1 1] Hit_Logic, if hited explode, activate item if it need, complete quest if it need, give damage and destroy self on end.
  (`NiagaraComponent.SetAsset` (`self.Niagara`) "/Game/TASK_Folder/Effects/Magic_Explode_Effet.Magic_Explode_Effet" true)
  (`GameplayStatics.ApplyDamage` _hitactor 27.5 null self)
  (`self.Activate_Interact_On_Impact` _hitactor _hitcomponent)
  (`KismetSystemLibrary.Delay` 1.0)
  (`self.K2_DestroyActor`))

(fn `Activate_Interact_On_Impact`
  (params (Hited_Actor :type "Actor Object Reference") (Hited_Component :type "PrimitiveComponent Object Reference"))
  (locals (Quest_System :type "Quest_System_Component_PR Object Reference"))
  (bind ((`Quest_ID` _quest_id) (`Quest_Locations` _quest_locations)) (break `Quest_Data` (`Quest_System_Component_PR.Get_Current_Quest_Data` (`local.Quest_System`))))
  (bind _ascustom_controller_bp (cast `/Game/TASK_Folder/Blueprints/Character/Custom_Controller_BP` (`GameplayStatics.GetPlayerController` 0)))
  (bind _quest_system (`Custom_Player_Controller_PR.Quest_System` _ascustom_controller_bp)
    (:`then`
      (set `local.Quest_System` _quest_system)
      (if (and (`KismetArrayLibrary.Array_Contains` (`Actor.Tags` Hited_Actor) "Quest_Obj") (`KismetSystemLibrary.DoesImplementInterface` Hited_Actor "/Script/UE5_Test_Task.Interact_Interface_PR"))
        (bind _returnvalue (message `Interact_Interface_PR.Get_Responsible_Quest` Hited_Actor))
        (bind _returnvalue_2 (message `Interact_Interface_PR.Get_Responsible_Location` Hited_Actor))
        (bind ((`Quest_ID` _quest_id_2)) (break `Quest_Data` _returnvalue))
        (bind (_value _returnvalue_3) (`BlueprintMapLibrary.Map_Find` _quest_locations _returnvalue_2))
        (if (and (`KismetStringLibrary.EqualEqual_StrStr` _quest_id_2 _quest_id) _returnvalue_3 (not _value) (`KismetStringLibrary.EqualEqual_StrStr` _quest_id_2 "Last Trouble") (or (== _returnvalue_2 (-17803.140038 -9151.874839 475.831489) :`ErrorTolerance` 0.1) (== _returnvalue_2 (265.465296 -5736.807198 388.182222) :`ErrorTolerance` 0.1)))
          (message `Interact_Interface_PR.On_Item_Interacted` Hited_Actor Hited_Component))))
    (:`else`)))

(fn `UserConstructionScript`)