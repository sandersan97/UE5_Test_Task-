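; Utility function library that loads saved game settings and applies them to graphics, audio and input.
; The load functions read a Game_Save_BP from the fixed settings slot or a given slot, creating and saving one if absent.
; LoadAndActivateSettingsSave loops through GameUserSettings setters, overrides Master, Music and SFX sound-mix volumes, and swaps the audio output device.
; It then pushes key mappings to Custom_Controller_BP and returns success.
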(fn `Load And Activate Settings Save`
  (params (On_Audio_Output_Swap_Completed :type "Delegate (by ref)"))
  (returns (Is_Succes :type Boolean))
  (locals (Settings_Save_LocalVar :type "/Game/TASK_Folder/Blueprints/Other/Game_Save_BP Object Reference"))
  (bind ((`Master_Volume_37_026B22754D4C388508B5EABB6C7ED836` _master_volume) (`Music_Volume_38_CC05E575456D54B0E385ECAD9695576F` _music_volume) (`SFX_Volume_39_06123CC343ECEC723C56B19985D3A75B` _sfx_volume) (`Dialogue_Volume_40_D32D02254F1F371D270A8391142F7C26` _dialogue_volume) (`Output_Mode_43_315CE92641485E15F5F170A6F261926D` _output_mode) (`KeyMappings_47_76E78F0E46F6FB39DFABA992AEC75F75` _keymappings)) (break `/Game/TASK_Folder/Blueprints/Struct/Game_Setings` (`/Game/TASK_Folder/Blueprints/Other/Game_Save_BP.Get_Game_Settings` (`local.Settings_Save_LocalVar`))))
  (bind ((`Window_Mode_18_0677E32448F15022F3E8B4B9E74B3E72` _window_mode) (`Display_Resolution_19_F2AD37214AE189AFB2215D9F5ED56221` _display_resolution) (`Frame_Rate_Limit_20_2FE4ACA14CA8442EE3FBE992E07F1FFE` _frame_rate_limit) (`ViewDistance_21_3F76517445E18D1E1CABF1932B35237B` _viewdistance) (`PostProcessing_22_0D6031AC46A4106EC02FE8A95248715C` _postprocessing) (`AntiAliasing_23_F427FA4847D300842EAEC992DC43A429` _antialiasing) (`TextureQuality_24_A70F3865425F69CC07F8CA85B4839498` _texturequality) (`ShadowQuality_25_603EB6CD416735DDE0BD3DA668732AD5` _shadowquality)) (break `/Game/TASK_Folder/Blueprints/Struct/Game_Setings` (`/Game/TASK_Folder/Blueprints/Other/Game_Save_BP.Get_Game_Settings` (`local.Settings_Save_LocalVar`))))
  (bind (_lefts _rights) (`KismetStringLibrary.Split` (`|GetEnumeratorNameAsString` _display_resolution) "x"))
  (bind (_issucces _save_result) (`self.Load_Settings_Save` null))
  (if _issucces
    (`/Engine/EditorBlueprintResources/StandardMacros.IsValid` _save_result
      (:`Is Valid`
        (set `local.Settings_Save_LocalVar` _save_result)
        (bind _returnvalue (`GameUserSettings.GetGameUserSettings`))
        (`/Engine/EditorBlueprintResources/StandardMacros.IsValid` _returnvalue
          (:`Is Valid`
            (for _index (range 9)
              ;[1 1 1] Activate Graphic Settings Settings.
              (switch `int` _index
                (:`0`
                  (bind _returnvalue_2 (`GameUserSettings.GetGameUserSettings`))
                  (`/Engine/EditorBlueprintResources/StandardMacros.IsValid` _returnvalue_2
                    (:`Is Valid`
                      (`GameUserSettings.SetFullscreenMode` _returnvalue_2 (select `/Game/TASK_Folder/Blueprints/Enums/Screen_Mode` _window_mode :`NewEnumerator0` "Windowed" :`NewEnumerator1` "Fullscreen" :!type "EWindowMode Enum")))))
                (:`1`
                  (bind _returnvalue_3 (`GameUserSettings.GetGameUserSettings`))
                  (`/Engine/EditorBlueprintResources/StandardMacros.IsValid` _returnvalue_3
                    (:`Is Valid`
                      (`GameUserSettings.SetScreenResolution` _returnvalue_3 (make `IntPoint` (`KismetStringLibrary.Conv_StringToInt` _lefts) (`KismetStringLibrary.Conv_StringToInt` _rights))))))
                (:`2`
                  (bind _returnvalue_4 (`GameUserSettings.GetGameUserSettings`))
                  (`/Engine/EditorBlueprintResources/StandardMacros.IsValid` _returnvalue_4
                    (:`Is Valid`
                      (`GameUserSettings.SetFrameRateLimit` _returnvalue_4 (select `/Game/TASK_Folder/Blueprints/Enums/Frame_Rate_Limit` _frame_rate_limit :`NewEnumerator0` 30.0 :`NewEnumerator1` 30.0 :`NewEnumerator2` 30.0 :`NewEnumerator3` 120.0 :`NewEnumerator4` 140.0 :`NewEnumerator5` 180.0 :`NewEnumerator6` 200.0 :!type "Float (single-precision)")))))
                (:`3`
                  (bind _returnvalue_5 (`GameUserSettings.GetGameUserSettings`))
                  (`/Engine/EditorBlueprintResources/StandardMacros.IsValid` _returnvalue_5
                    (:`Is Valid`
                      (`GameUserSettings.SetViewDistanceQuality` _returnvalue_5 (select `/Game/TASK_Folder/Blueprints/Enums/Settings_Grade` _viewdistance :`NewEnumerator1` 1 :`NewEnumerator2` 2 :`NewEnumerator3` 3)))))
                (:`4`
                  (bind _returnvalue_6 (`GameUserSettings.GetGameUserSettings`))
                  (`/Engine/EditorBlueprintResources/StandardMacros.IsValid` _returnvalue_6
                    (:`Is Valid`
                      (`GameUserSettings.SetPostProcessingQuality` _returnvalue_6 (select `/Game/TASK_Folder/Blueprints/Enums/Settings_Grade` _postprocessing :`NewEnumerator1` 1 :`NewEnumerator2` 2 :`NewEnumerator3` 3)))))
                (:`5`
                  (bind _returnvalue_7 (`GameUserSettings.GetGameUserSettings`))
                  (`/Engine/EditorBlueprintResources/StandardMacros.IsValid` _returnvalue_7
                    (:`Is Valid`
                      (`GameUserSettings.SetAntiAliasingQuality` _returnvalue_7 (select `/Game/TASK_Folder/Blueprints/Enums/Settings_Grade` _antialiasing :`NewEnumerator1` 1 :`NewEnumerator2` 2 :`NewEnumerator3` 3)))))
                (:`6`
                  (bind _returnvalue_8 (`GameUserSettings.GetGameUserSettings`))
                  (`/Engine/EditorBlueprintResources/StandardMacros.IsValid` _returnvalue_8
                    (:`Is Valid`
                      (`GameUserSettings.SetTextureQuality` _returnvalue_8 (select `/Game/TASK_Folder/Blueprints/Enums/Settings_Grade` _texturequality :`NewEnumerator1` 1 :`NewEnumerator2` 2 :`NewEnumerator3` 3)))))
                (:`7`
                  (bind _returnvalue_9 (`GameUserSettings.GetGameUserSettings`))
                  (`/Engine/EditorBlueprintResources/StandardMacros.IsValid` _returnvalue_9
                    (:`Is Valid`
                      (`GameUserSettings.SetShadingQuality` _returnvalue_9 (select `/Game/TASK_Folder/Blueprints/Enums/Settings_Grade` _shadowquality :`NewEnumerator1` 1 :`NewEnumerator2` 2 :`NewEnumerator3` 3)))))))
            (`GameUserSettings.ApplySettings` _returnvalue false)
            ;[1 1 1] Activate Audio Settings
            (for _index_2 (range 5)
              (if (< _index_2 3)
                (`GameplayStatics.SetSoundMixClassOverride` null (select `int` _index_2 :`0` "/Game/TASK_Folder/Sounds/Clases/Master_Mix_Sound.Master_Mix_Sound" :`1` "/Game/TASK_Folder/Sounds/Clases/Music_Mix_Sound.Music_Mix_Sound" :`2` "/Game/TASK_Folder/Sounds/Clases/SFX_Mix_Sound.SFX_Mix_Sound" :`3` "/Game/TASK_Folder/Sounds/Clases/Dialogue_Mix_Sound.Dialogue_Mix_Sound" :!type "SoundMix Object Reference") (select `int` _index_2 :`0` "/Game/TASK_Folder/Sounds/Clases/Master_Class_Sound.Master_Class_Sound" :`1` "/Game/TASK_Folder/Sounds/Clases/Music_Class_Sound.Music_Class_Sound" :`2` "/Game/TASK_Folder/Sounds/Clases/SFX_Class_Sound.SFX_Class_Sound" :`3` "/Game/TASK_Folder/Sounds/Clases/Dialogue_Class_Sound.Dialogue_Class_Sound" :!type "SoundClass Object Reference") (select `int` _index_2 :`0` _master_volume :`1` _music_volume :`2` _sfx_volume :`3` _dialogue_volume :!type "Float (single-precision)"))
                (elif (not (`KismetStringLibrary.IsEmpty` _output_mode))
                  (`AudioMixerBlueprintLibrary.SwapAudioOutputDevice` null _output_mode On_Audio_Output_Swap_Completed))))
            ;[1 1 1] Update and Activate Input Settings
            (bind _ascustom_controller_bp (cast `/Game/TASK_Folder/Blueprints/Character/Custom_Controller_BP` (`GameplayStatics.GetPlayerController` null))
              (:`then`
                (`/Game/TASK_Folder/Blueprints/Character/Custom_Controller_BP.Set_Input_Mappings` _ascustom_controller_bp _keymappings)
                (`/Game/TASK_Folder/Blueprints/Character/Custom_Controller_BP.Update Input Mappings` _ascustom_controller_bp)
                (return true))
              (:`CastFailed`
                (return false))))
          (:`Is Not Valid`
            (return false))))
      (:`Is Not Valid`
        _)))
  (return false))

(fn `Load_CustomSave`
  (params (SlotName :type String) (UserIndex :type Integer))
  (returns (IsSucces :type Boolean) (Save_Result :type "/Game/TASK_Folder/Blueprints/Other/Game_Save_BP Object Reference"))
  (locals (Settings_Save :type "/Game/TASK_Folder/Blueprints/Other/Game_Save_BP Object Reference"))
  (bind _returnvalue (`GameplayStatics.DoesSaveGameExist` SlotName UserIndex))
  (if _returnvalue
    (bind _returnvalue_2 (`GameplayStatics.LoadGameFromSlot` SlotName UserIndex))
    (bind _asgame_save_bp (cast `/Game/TASK_Folder/Blueprints/Other/Game_Save_BP` _returnvalue_2)
      (:`then`
        (bind _output_get (set `local.Settings_Save` _asgame_save_bp))
        (return true _output_get))
      (:`CastFailed`
        (return false null)))
    (else
      (bind _returnvalue_3 (`GameplayStatics.CreateSaveGameObject` "/Game/TASK_Folder/Blueprints/Other/Game_Save_BP.Game_Save_BP_C"))
      (bind _output_get_2 (set `local.Settings_Save` _returnvalue_3))
      (bind _returnvalue_4 (`GameplayStatics.SaveGameToSlot` _output_get_2 SlotName UserIndex))
      (return _returnvalue_4 _output_get_2))))

(fn `Load_Settings_Save`
  (returns (IsSucces :type Boolean) (Save_Result :type "/Game/TASK_Folder/Blueprints/Other/Game_Save_BP Object Reference"))
  (locals (Settings_Save :type "/Game/TASK_Folder/Blueprints/Other/Game_Save_BP Object Reference"))
  (bind _returnvalue (`GameplayStatics.DoesSaveGameExist` "Game_Settings"))
  (if _returnvalue
    (bind _returnvalue_2 (`GameplayStatics.LoadGameFromSlot` "Game_Settings"))
    (bind _asgame_save_bp (cast `/Game/TASK_Folder/Blueprints/Other/Game_Save_BP` _returnvalue_2)
      (:`then`
        (bind _output_get (set `local.Settings_Save` _asgame_save_bp))
        (return true _output_get))
      (:`CastFailed`
        (return false null)))
    (else
      (bind _returnvalue_3 (`GameplayStatics.CreateSaveGameObject` "/Game/TASK_Folder/Blueprints/Other/Game_Save_BP.Game_Save_BP_C"))
      (bind _output_get_2 (set `local.Settings_Save` _returnvalue_3))
      (bind _returnvalue_4 (`GameplayStatics.SaveGameToSlot` _output_get_2 "Game_Settings"))
      (return _returnvalue_4 _output_get_2))))